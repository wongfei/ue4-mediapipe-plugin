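; MediaPipe pipeline wrapper Blueprint that controls a Pipeline object and provides debug drawing for its tracking output.
; StartPipeline applies the overlay flag and starts only when EnableAutoStart is set, alongside functions to stop it and assign graph nodes.
; Debug helpers draw the camera and world origins, plus a valid observer's detected landmarks with a box marking landmark 0.
; BeginPlay, EndPlay and Tick are empty, so nothing here calls these functions.
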(event `self.ReceiveBeginPlay`)

(event `self.ReceiveEndPlay`
  (params (EndPlayReason :type "EEndPlayReason Enum" :default "Destroyed")))

(event `self.ReceiveTick`
  (params (DeltaSeconds :type "Float (single-precision)")))

(fn `DrawCameraOrigin`
  (bind _cameraorigin (`self.CameraOrigin`))
  (`KismetSystemLibrary.DrawDebugCoordinateSystem` _cameraorigin (struct) 10.0)
  (`KismetSystemLibrary.DrawDebugBox` (+ _cameraorigin (0.0 50.0 -50.0)) (5.0 50.0 50.0)))

(fn `DrawLandmarks`
  (params (Observer :type "MediaPipeLandmarkObserverComponent Object Reference") (ObjectId :type Integer) (Origin :type "Vector Structure") (PrimitiveScale :type "Float (double-precision)") (PrimitiveColor :type "LinearColor Structure"))
  (`/Engine/EditorBlueprintResources/StandardMacros.IsValid` Observer
    (:`Is Valid`
      (if (`MediaPipeObserverComponent.HaveDetections` Observer)
        (`MediaPipeLandmarkObserverComponent.DrawDebugLandmarks` Observer ObjectId (`KismetMathLibrary.MakeTransform` Origin) PrimitiveScale PrimitiveColor)
        (`KismetSystemLibrary.DrawDebugBox` (+ Origin (`.Pos` (break `MediaPipeLandmark` (`MediaPipeLandmarkObserverComponent.GetLandmark` Observer ObjectId 0)))) (1.0 1.0 1.0) PrimitiveColor)))))

(fn `DrawWorldOrigin`
  (bind _worldorigin (`self.WorldOrigin`))
  (`KismetSystemLibrary.DrawDebugCoordinateSystem` _worldorigin (struct) 10.0)
  (`KismetSystemLibrary.DrawDebugBox` _worldorigin (100.0 100.0 100.0) (struct :`A` 1.0)))

(fn `SetGraphNode`
  (params (Node :type String))
  (set `MediaPipePipelineComponent.GraphNodes` (`|MakeArray` Node) (`self.Pipeline`)))

(fn `SetGraphNodes`
  (params (Nodes :type "Array of String"))
  (set `MediaPipePipelineComponent.GraphNodes` Nodes (`self.Pipeline`)))

(fn `StartPipeline`
  (if (`self.EnableAutoStart`)
    (set `MediaPipePipelineComponent.bEnableOverlay` (`self.EnableOverlay`) (`self.Pipeline`))
    (`MediaPipePipelineComponent.Start` (`self.Pipeline`))))

(fn `StopPipeline`
  (`MediaPipePipelineComponent.Stop` (`self.Pipeline`)))

(fn `UserConstructionScript`)