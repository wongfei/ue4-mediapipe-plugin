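; MediaPipe 3D face geometry actor that visualizes a tracked face mesh with debug drawing.
; The pipeline starts on BeginPlay and stops on EndPlay.
; Each tick draws the world origin and, if a face is detected, the first mesh's vertices using its pose transform, plus a small box at vertex 0 transformed by that pose.
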(event `self.ReceiveBeginPlay`
  (`self.StartPipeline`))

(event `self.ReceiveEndPlay`
  (params (EndPlayReason :type "EEndPlayReason Enum" :default "Destroyed"))
  (`self.StopPipeline`))

(event `self.ReceiveTick`
  (params (DeltaSeconds :type "Float (single-precision)"))
  (`self.DrawWorldOrigin`)
  (`self.DrawFaceMesh3D` 0))

(fn `DrawFaceMesh3D`
  (params (MeshId :type Integer))
  (bind _facemesh (`self.FaceMesh`))
  (bind _pose (break `MediaPipeFaceMesh` (`MediaPipeFaceMeshObserverComponent.GetMesh` _facemesh MeshId)))
  (if (< MeshId (`MediaPipeObserverComponent.GetNumDetections` (`self.FaceMesh`)))
    (`MediaPipeFaceMeshObserverComponent.DrawDebugMeshVertices` _facemesh 0 _pose 3.0 (struct :`G` 1.0 :`B` 0.128237 :`A` 1.0))
    (`KismetSystemLibrary.DrawDebugBox` (`KismetMathLibrary.TransformLocation` _pose (`.Pos` (break `MediaPipeVertex` (`MediaPipeFaceMeshObserverComponent.GetMeshVertex` (`self.FaceMesh`) MeshId 0)))) (1.0 1.0 1.0) (struct :`G` 1.0 :`A` 1.0))))

(fn `UserConstructionScript`)